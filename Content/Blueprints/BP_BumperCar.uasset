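; Bumper car Blueprint that applies raycast spring suspension to a physics cube.
; Each tick, TraceRays casts short downward line traces from four corner components and collects the hits.
; SuspensionFromRay feeds hit time and the corner's vertical velocity into SpringDampening, then applies the vertical result as an impulse on the cube at that corner.
; Traces, printed values and arrows provide per-frame debug output.
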(event EventTick
  (params (DeltaSeconds :type Float%20%28single-precision%29))
  (bind _raytracehit (CallFunction|TraceRays))
  (for _array_element _raytracehit
    (CallFunction|SuspensionfromRay _array_element)))

(fn ConstructionScript)

(fn TraceRays
  (bind _corner4 (Variables|Default|GetCorner4))
  (bind _corner1 (Variables|Default|GetCorner1))
  (bind _corner2 (Variables|Default|GetCorner2))
  (bind _corner3 (Variables|Default|GetCorner3))
  (bind _returnvalue (Transformation|GetWorldLocation _corner4))
  (bind _returnvalue_2 (Transformation|GetWorldLocation _corner1))
  (bind _returnvalue_3 (Transformation|GetWorldLocation _corner2))
  (bind _returnvalue_4 (Transformation|GetWorldLocation _corner3))
  (bind (_x _y _z) (Math|Vector|BreakVector _returnvalue_2))
  (bind (_x_2 _y_2 _z_2) (Math|Vector|BreakVector _returnvalue_3))
  (bind (_x_3 _y_3 _z_3) (Math|Vector|BreakVector _returnvalue))
  (bind (_x_4 _y_4 _z_4) (Math|Vector|BreakVector _returnvalue_4))
  (Utilities|FlowControl|Sequence
    (:then_0
      (bind _outhit (Collision|LineTraceByChannel _returnvalue_2 (Math|Vector|MakeVector _x _y (- _z 1e+02)) "TraceTypeQuery1" false 0 "ForOneFrame"))
      (Utilities|Array|Add (LocalVariables|Gethits) (Utilities|Struct|MakeS_RayCast _outhit _returnvalue_2 (Variables|Default|GetCorner1))))
    (:then_1
      (bind _outhit_2 (Collision|LineTraceByChannel _returnvalue_3 (Math|Vector|MakeVector _x_2 _y_2 (- _z_2 1e+02)) "TraceTypeQuery1" false 0 "ForOneFrame"))
      (Utilities|Array|Add (LocalVariables|Gethits) (Utilities|Struct|MakeS_RayCast _outhit_2 _returnvalue_3 (Variables|Default|GetCorner2))))
    (:then_2
      (bind _outhit_3 (Collision|LineTraceByChannel _returnvalue_4 (Math|Vector|MakeVector _x_4 _y_4 (- _z_4 1e+02)) "TraceTypeQuery1" false 0 "ForOneFrame"))
      (Utilities|Array|Add (LocalVariables|Gethits) (Utilities|Struct|MakeS_RayCast _outhit_3 _returnvalue_4 (Variables|Default|GetCorner3))))
    (:then_3
      (bind _outhit_4 (Collision|LineTraceByChannel _returnvalue (Math|Vector|MakeVector _x_3 _y_3 (- _z_3 1e+02)) "TraceTypeQuery1" false 0 "ForOneFrame"))
      (Utilities|Array|Add (LocalVariables|Gethits) (Utilities|Struct|MakeS_RayCast _outhit_4 _returnvalue (Variables|Default|GetCorner4)))
      (return (LocalVariables|Gethits)))))

(fn SuspensionfromRay
  (params (hit :type S%20Ray%20Cast%20Structure))
  (bind _returnvalue (Transformation|GetComponentVelocity (.positionmesh hit)))
  (bind _returnvalue_2 (Transformation|GetWorldLocation (.positionmesh hit)))
  (bind _dampingspeed (Utilities|SpringDampening 5e+02 (.time (.hit hit)) 5e+02 (.z _returnvalue)))
  (Development|PrintString (Utilities|String|ToString(Float) _dampingspeed) true true "(R=0.000000,G=0.660000,B=1.000000,A=1.000000)" 0.0)
  (Physics|AddImpulseatLocation (Variables|Default|GetCube) (Math|Vector|MakeVector 0.0 0.0 _dampingspeed) (.initiallocation hit) "None")
  (Rendering|Debug|DrawDebugArrow :LineStart (Math|Vector|MakeVector (.x _returnvalue_2) (.y _returnvalue_2) (.z _returnvalue_2)) :LineEnd (Math|Vector|MakeVector (.x _returnvalue_2) (.y _returnvalue_2) (+ (.z _returnvalue_2) _dampingspeed))))
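; BP_BumperCarTrigger is a box trigger that puts the player into a random bumper car.
; On player overlap it picks from all BP_BumperCarPawn actors, stores the original pawn cached at BeginPlay in PawnPlayer, possesses a car and adds the IMC_BumperCar input context.
; The random pick feeds both steps separately, so the car given PawnPlayer can differ from the possessed one.
; End overlap only checks for the player and does nothing.
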(event OnComponentBeginOverlap(Box)
  (params (OverlappedComponent :type Primitive%20Component%20Object%20Reference) (OtherActor :type Actor%20Object%20Reference) (OtherComp :type Primitive%20Component%20Object%20Reference) (OtherBodyIndex :type Integer) (bFromSweep :type Boolean) (SweepResult :type Hit%20Result%20Structure%20%28by%20ref%29))
  (bind _returnvalue (Game|GetPlayerController 0))
  (if (== OtherActor (Game|Player|GetPlayerPawn 0))
    (bind _outactors (Actor|GetAllActorsOfClass "/Game/Blueprints/BP_BumperCarPawn.BP_BumperCarPawn_C"))
    (Variables|/Game/Blueprints/BP_BumperCarPawn.BP_BumperCarPawn_C|SetpawnPlayer (.OutItem (Utilities|Array|Random _outactors)) (Variables|Default|GetPlayerPawn))
    (Pawn|Possess _returnvalue (.OutItem (Utilities|Array|Random _outactors)))
    (Input|AddMappingContext (PlayerController|LocalPlayerSubsystems|GetEnhancedInputLocalPlayerSubsystem _returnvalue) "/Game/imc/IMC_BumperCar.IMC_BumperCar" 0 "(bIgnoreAllPressedKeysUntilRelease=True,bForceImmediately=False,bNotifyUserSettings=False)")))

(event OnComponentEndOverlap(Box)
  (params (OverlappedComponent :type Primitive%20Component%20Object%20Reference) (OtherActor :type Actor%20Object%20Reference) (OtherComp :type Primitive%20Component%20Object%20Reference) (OtherBodyIndex :type Integer))
  (if (== OtherActor (Game|Player|GetPlayerPawn 0))
    _))

(event EventBeginPlay
  (Variables|Default|SetPlayerPawn (Game|Player|GetPlayerPawn 0)))

(fn ConstructionScript)
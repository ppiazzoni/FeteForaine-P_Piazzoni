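; BP_NPC is an actor that wanders between randomly chosen BP_TargetPoint actors gathered at BeginPlay.
; Move branches on a random point's Type: Regular moves and repeats on success or failure, while Creation only delays, ending the loop.
; Destruction destroys the NPC immediately after issuing AIMoveTo, without awaiting arrival.
; The pure Random node is re-evaluated per use, so the destination can differ from the point whose type is checked.
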(event Custom|Move
  (bind _self self)
  (bind _target (Variables|Default|GetTarget))
  (bind _outitem (Utilities|Array|Random _target))
  (switch Utilities|FlowControl|Switch|SwitchonE_Targetpoint (Variables|/Game/Blueprints/BP_TargetPoint.BP_TargetPoint_C|GetType _outitem)
    (:NewEnumerator0
      (Utilities|FlowControl|Delay 0.2))
    (:NewEnumerator1
      (AI|AIMoveTo _self "0, 0, 0" _outitem 5.0 false
        (:then
          (Actor|DestroyActor))))
    (:NewEnumerator2
      (AI|AIMoveTo _self "0, 0, 0" _outitem 5.0 false
        (:OnSuccess
          _)
        (:OnFail
          _))
      (CallFunction|Move))))

(event EventBeginPlay
  (bind _outactors (Actor|GetAllActorsOfClass "/Game/Blueprints/BP_TargetPoint.BP_TargetPoint_C"))
  (Variables|Default|SetTarget _outactors)
  (CallFunction|Move))

(event Collision|EventActorBeginOverlap
  (params (OtherActor :type Actor%20Object%20Reference)))

(event EventTick
  (params (DeltaSeconds :type Float%20%28single-precision%29)))

(fn ConstructionScript)
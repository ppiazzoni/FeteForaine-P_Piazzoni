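; BP_Shoot fires physics-driven BP_Ball actors from the camera toward the mouse cursor with a hold-and-release power shot.
; While the left mouse button is held and CanShoot is true, accumulated hold time drives an oscillating sine power value on ShootBar.
; On release, a cursor line trace sets the aim, and the spawned ball receives an impulse scaled by that same power and ShootSpeed.
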(event Custom|ReleasedLMB
  (params (HeldTime :type Float%20%28double-precision%29))
  (bind _returnvalue (Game|GetPlayerController 0))
  (bind (_worldlocation _worlddirection) (Game|Player|ConvertMouseLocationToWorldSpace _returnvalue))
  (if (Variables|Default|GetcanShoot)
    (bind _outhit (Collision|LineTraceByChannel _worldlocation (+ _worldlocation (* _worlddirection 9e+08)) "TraceTypeQuery1" false 0 "None"))
    (bind _returnvalue_2 (Game|SpawnActorfromClass "/Game/Blueprints/BP_Ball.BP_Ball_C" (Math|Transform|MakeTransform (Camera|GetCameraLocation (Game|GetPlayerCameraManager 0)) "0, 0, 0" (Math|Conversions|ToVector(Float) (Math|Random|RandomFloatinRange 0.1 0.1))) "Undefined" "MultiplyWithRoot" 0 0))
    (Collision|SetCollisionEnabled (Variables|/Game/Blueprints/BP_Ball.BP_Ball_C|GetSphere _returnvalue_2) "PhysicsOnly")
    (Physics|AddImpulse (Variables|/Game/Blueprints/BP_Ball.BP_Ball_C|GetSphere _returnvalue_2) (* (Math|Vector|ClampVectorSize (- (.Location (Collision|BreakHitResult _outhit)) (Transformation|GetWorldLocation (Variables|/Game/Blueprints/BP_Ball.BP_Ball_C|GetSphere _returnvalue_2))) 0.0 1.0) (* (/ (+ (Math|Trig|Sin(Degrees) (+ (* HeldTime 1e+02) 5.0)) 1.0) 2.0) (Variables|Default|GetShootSpeed))) "None" false)))

(event EventBeginPlay)

(event EventTick
  (params (DeltaSeconds :type Float%20%28single-precision%29))
  (if (Variables|Default|GetholdingLMB)
    (if (Variables|Default|GetcanShoot)
      (bind _output_get (Variables|Default|SetlmbHeldTime (+ DeltaSeconds (Variables|Default|GetlmbHeldTime))))
      (Variables|/Game/Widget/W_ShootBar.W_ShootBar_C|SetProgressBarPercent (Variables|Default|GetshootBar) (/ (+ (Math|Trig|Sin(Degrees) (+ (* _output_get 1e+02) 5.0)) 1.0) 2.0)))))

(event Input|MouseEvents|LeftMouseButton
  (params (Key :type Key%20Structure :default "None"))
  (:Pressed
    (Variables|Default|SetholdingLMB true))
  (:Released
    (Variables|Default|SetholdingLMB false)
    (CallFunction|ReleasedLMB (Variables|Default|GetlmbHeldTime))
    (Variables|Default|SetlmbHeldTime 0.0)))